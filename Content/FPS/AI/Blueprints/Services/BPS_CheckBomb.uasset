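; BPS_CheckBomb is a behavior tree service that points the AI at the NPC referenced by the Protect game state.
; On search start it casts the game state to BP_Protect_GS and, if NPCRef is valid, raises the bomb-interaction blackboard flag.
; It also writes a location offset along world Y from that NPC and stores the NPC as Enemy.
; Two inner branches are hardwired to true.
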(event `self.ReceiveSearchStartAI`
  (params (OwnerController :type "AIController Object Reference") (ControlledPawn :type "Pawn Object Reference"))
  (bind _asbp_protect_gs (cast `/Game/FPS/Blueprints/GameModes/Protect/BP_Protect_GS` (`GameplayStatics.GetGameState`)))
  (bind _npcref (`/Game/FPS/Blueprints/GameModes/Protect/BP_Protect_GS.NPCRef` _asbp_protect_gs))
  (`/Engine/EditorBlueprintResources/StandardMacros.IsValid` _npcref
    (:`Is Valid`
      (if true
        (if true
          (`BTFunctionLibrary.SetBlackboardValueAsBool` (`self.InteractBombKey`) true)
          (bind (_returnvalue_x _returnvalue_y _returnvalue_z) (`KismetMathLibrary.BreakVector` (`Actor.K2_GetActorLocation` _npcref)))
          (`BTFunctionLibrary.SetBlackboardValueAsVector` (`self.LocationKey`) (`KismetMathLibrary.MakeVector` _returnvalue_x (+ _returnvalue_y 200.0) _returnvalue_z))
          (`BTFunctionLibrary.SetBlackboardValueAsObject` (`self.Enemy`) _npcref))))))