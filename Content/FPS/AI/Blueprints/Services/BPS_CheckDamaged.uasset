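; Behavior tree service that watches an AI-controlled player character's health and switches its targeting state.
; Each tick, if HP is below maximum, it sets the Damaged blackboard key and has the AI controller clear its enemy.
; At full health, it writes the Protect game state's NPC character to the Enemy key when that reference is valid.
; The service never resets Damaged to false.
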(event `self.ReceiveTickAI`
  (params (OwnerController :type "AIController Object Reference") (ControlledPawn :type "Pawn Object Reference") (DeltaSeconds :type "Float (single-precision)"))
  (bind _asbp_player_character (cast `/Game/FPS/Blueprints/CharacterAndClasses/BP_PlayerCharacter` ControlledPawn))
  (bind _healthcomponent (`/Game/FPS/Blueprints/CharacterAndClasses/BP_PlayerCharacter.HealthComponent` _asbp_player_character))
  (if (< (`/Game/FPS/Blueprints/HealthComponent/BP_HealthComponent.HP` _healthcomponent) (`/Game/FPS/Blueprints/HealthComponent/BP_HealthComponent.MaxHP` _healthcomponent))
    (`BTFunctionLibrary.SetBlackboardValueAsBool` (`self.Damaged`) true)
    (bind _asbp_ai_player_controller (cast `/Game/FPS/AI/Controllers/BP_AI_PlayerController` OwnerController))
    (`/Game/FPS/AI/Controllers/BP_AI_PlayerController.ClearEnemy` _asbp_ai_player_controller)
    (else
      (bind _asbp_protect_gs (cast `/Game/FPS/Blueprints/GameModes/Protect/BP_Protect_GS` (`GameplayStatics.GetGameState`)))
      (bind _npccharacterref (`/Game/FPS/Blueprints/GameModes/Protect/BP_Protect_GS.NPCCharacterRef` _asbp_protect_gs))
      (`/Engine/EditorBlueprintResources/StandardMacros.IsValid` _npccharacterref
        (:`Is Valid`
          (`BTFunctionLibrary.SetBlackboardValueAsObject` (`self.Enemy`) _npccharacterref))))))