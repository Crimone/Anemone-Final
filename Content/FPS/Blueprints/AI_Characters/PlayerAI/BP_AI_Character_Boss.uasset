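; Boss AI character whose health is mirrored to the Protect mode game state.
; It spawns with a random machinegun or shotgun plus a pistol, and its melee action drops a gas grenade whenever that skill is off cooldown.
; It takes one-tenth damage, and a first hit, depending on the attacker's team, switches it to BT_Rush against that attacker.
; BotShoot multi-traces a spread cone at the blackboard enemy, weakening damage with each successive hit.
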(event `self.Server_BotEquipWeapon`
  (bind _primaryweapon (`self.PrimaryWeapon`))
  ;[1 1 1] Weapon
  (`/Engine/EditorBlueprintResources/StandardMacros.IsValid` (`self.CurrentWeapon`)
    (:`Is Not Valid`
      (bind _output_get (set `self.PrimaryWeaponToSpawn` (select `int` (`KismetMathLibrary.RandomIntegerInRange` 0 1) :`0` "/Game/FPS/Blueprints/Weapons/BP_Machinegun_Weapon.BP_Machinegun_Weapon_C" :`1` "/Game/FPS/Blueprints/Weapons/BP_Shotgun_Weapon.BP_Shotgun_Weapon_C" :!type "/Game/FPS/Blueprints/Weapons/BP_BaseWeapon Class Reference")))
      (set `self.EquippedWeapon` (`.WeaponType` (defaults `Object` _output_get)))
      (`self.EquipWeapon` _output_get 0 true true)
      (`self.EquipWeapon` "/Game/FPS/Blueprints/Weapons/BP_Pistol_02_Weapon.BP_Pistol_02_Weapon_C")
      (set `self.CurrentWeapon` _primaryweapon)
      (`self.SetNetDormancy` _primaryweapon "DORM_Awake")
      (`self.SetWeaponVisibility` (`self.SecondaryWeapon`))
      (bind _asbp_protect_gs (cast `/Game/FPS/Blueprints/GameModes/Protect/BP_Protect_GS` (`GameplayStatics.GetGameState`)))
      (set `/Game/FPS/Blueprints/GameModes/Protect/BP_Protect_GS.BossHealth` 100.0 _asbp_protect_gs))))

(event `/Game/FPS/Blueprints/Interfaces/iPawnActions.AIUseMelee`
  ;[1 1 1] AI Melee
  (if (`self.SkillCoolingDown`)
    (`self.AI_Melee`)
    (`self.Multicast_PlayMeleeMontage`)
    (else
      (set `self.bPerformingAction` true)
      (bind _output_get (set `self.bUsingLethal` true))
      (`self.Server_SetUsingLethal` _output_get)
      (`|SpawnActorFromClass` "/Game/FPS/Blueprints/Grenade/BP_GasGrenade.BP_GasGrenade_C" (`KismetMathLibrary.MakeTransform` (`self.K2_GetActorLocation` self) (`KismetMathLibrary.MakeRotator` 0.0)) "AdjustIfPossibleButAlwaysSpawn" "OverrideRootScale" null 10.0 0.0 self)
      (set `self.SkillCoolingDown` true)
      (`KismetSystemLibrary.K2_SetTimerDelegate` (delegate `RefreshCD`) 10.0)
      (bind _output_get_2 (set `self.bUsingLethal` false))
      (`self.Server_SetUsingLethal` _output_get_2))))

(event `RefreshCD`
  (set `self.SkillCoolingDown` false))

(event `self.ReceiveAnyDamage`
  (params (Damage :type "Float (single-precision)") (DamageType :type "DamageType Object Reference") (InstigatedBy :type "Controller Object Reference") (DamageCauser :type "Actor Object Reference"))
  (bind _returnvalue (`Controller.K2_GetPawn` InstigatedBy))
  (bind _returnvalue_2 (* 0.1 Damage))
  (bind _returnvalue_3 (`AIBlueprintHelperLibrary.GetAIController` self))
  (bind _returnvalue_4 (`AIBlueprintHelperLibrary.GetAIController` self))
  ;[1 1 1] AnyDamage
  ;;[0.119 1 0] Handle Friend Damage
  (`/Engine/EditorBlueprintResources/StandardMacros.IsValid` InstigatedBy
    (:`Is Valid`
      (bind _playerstate (`Controller.PlayerState` InstigatedBy)
        (:`then`
          (bind _team (message `/Game/FPS/Blueprints/Interfaces/iPlayerState.GetTeam` _playerstate))
          (if (`KismetMathLibrary.Conv_IntToBool` _team)
            _
            (elif (not (`self.bDamaged`))
              ;;[0 0.1208 1] Change BT and Enemy
              (`AIController.RunBehaviorTree` _returnvalue_3 "/Game/FPS/AI/BehaviorTree/Rush/BT_Rush.BT_Rush")
              (bind _asbp_ai_player_controller (cast `/Game/FPS/AI/Controllers/BP_AI_PlayerController` _returnvalue_3))
              (bind _asbp_base_character (cast `/Game/FPS/Blueprints/CharacterAndClasses/BP_BaseCharacter` (`Controller.K2_GetPawn` InstigatedBy)))
              (`/Game/FPS/AI/Controllers/BP_AI_PlayerController.SetEnemy` _asbp_ai_player_controller _asbp_base_character)
              (set `self.bDamaged` true))))
        (:`else`
          _)))
    (:`Is Not Valid`
      _))
  ;;[1 0 0.4515] Handle Damage
  (`self.On DamageTaken` _returnvalue_2 DamageType InstigatedBy DamageCauser)
  (`|ExecutionSequence`
    (:`then_0`
      (if (`self.bDead`)
        (bind _asbp_protect_gs (cast `/Game/FPS/Blueprints/GameModes/Protect/BP_Protect_GS` (`GameplayStatics.GetGameState`)))
        (set `/Game/FPS/Blueprints/GameModes/Protect/BP_Protect_GS.BossHealth` -1.0 _asbp_protect_gs)
        (`/Engine/EditorBlueprintResources/StandardMacros.IsValid` _returnvalue_4
          (:`Is Valid`
            (`Controller.UnPossess` _returnvalue_4)
            (`KismetSystemLibrary.Delay` 10.0)
            (`self.K2_DestroyActor`)))))
    (:`then_1`
      (`/Engine/EditorBlueprintResources/StandardMacros.IsValid` InstigatedBy
        (:`Is Valid`
          (if (> Damage 5.0)
            (`/Engine/EditorBlueprintResources/StandardMacros.IsValid` _returnvalue
              (:`Is Valid`
                (`AISense_Damage.ReportDamageEvent` self _returnvalue Damage (`self.K2_GetActorLocation` _returnvalue))
                (bind _asbp_protect_gs_2 (cast `/Game/FPS/Blueprints/GameModes/Protect/BP_Protect_GS` (`GameplayStatics.GetGameState`)))
                (set `/Game/FPS/Blueprints/GameModes/Protect/BP_Protect_GS.BossHealth` (- (`/Game/FPS/Blueprints/GameModes/Protect/BP_Protect_GS.BossHealth` _asbp_protect_gs_2) _returnvalue_2) _asbp_protect_gs_2)))))))))

(fn `BotShoot`
  (bind _enemy (`self.Enemy`))
  (bind _returnvalue (`AIBlueprintHelperLibrary.GetBlackboard` self))
  (bind _returnvalue_2 (`SceneComponent.K2_GetComponentLocation` (`/Game/FPS/Blueprints/Weapons/BP_BaseWeapon.MeshFPP` (`self.CurrentWeapon`))))
  (bind _returnvalue_3 (`BlackboardComponent.GetValueAsObject` _returnvalue _enemy))
  (bind _asbp_player_character (cast `/Game/FPS/Blueprints/CharacterAndClasses/BP_PlayerCharacter` _returnvalue_3 :!pure true))
  (`/Engine/EditorBlueprintResources/StandardMacros.IsValid` _returnvalue
    (:`Is Valid`
      (`/Engine/EditorBlueprintResources/StandardMacros.IsValid` _returnvalue_3
        (:`Is Valid`
          (if (not (`/Game/FPS/Blueprints/CharacterAndClasses/BP_BaseCharacter.bDead` _asbp_player_character))
            (bind _outhits (`KismetSystemLibrary.LineTraceMulti` _returnvalue_2 (+ _returnvalue_2 (* (`KismetMathLibrary.RandomUnitVectorInConeInRadians` (`KismetMathLibrary.GetDirectionUnitVector` _returnvalue_2 (`self.K2_GetActorLocation` _asbp_player_character)) (`self.BotWeaponSpread`)) 6000.0)) "TraceTypeQuery4"))
            (for (_array_element _array_index) _outhits
              (`/Game/FPS/Blueprints/Weapons/BP_BaseWeapon.Server_PlayImpactEffects` (`self.CurrentWeapon`) _array_element)
              (bind (_bblockinghit _binitialoverlap _time _distance _location _impactpoint _normal _impactnormal _physmat _hitactor) (`GameplayStatics.BreakHitResult` _array_element))
              (`/Engine/EditorBlueprintResources/StandardMacros.IsValid` _hitactor
                (:`Is Valid`
                  (`/Engine/EditorBlueprintResources/StandardMacros.IsValid` (`self.GetComponentByClass` _hitactor "/Game/FPS/Blueprints/HealthComponent/BP_HealthComponent.BP_HealthComponent_C")
                    (:`Is Valid`
                      (`/Game/FPS/Blueprints/Weapons/BP_BaseWeapon.Server_InstantBulletHit` (`self.CurrentWeapon`) _array_element (/ 0.2 (`KismetMathLibrary.Conv_IntToDouble` (+ _array_index 1))) self))))))
            (`/Game/FPS/Blueprints/Weapons/BP_BaseWeapon.Server_PlayShotEffects` (`self.CurrentWeapon`))
            (else
              (`BlackboardComponent.SetValueAsObject` _returnvalue _enemy null :!label _label)
              (`self.StopShoting `))))
        (:`Is Not Valid`
          (goto _label))))))

(fn `UserConstructionScript`
  (`parent.UserConstructionScript`))