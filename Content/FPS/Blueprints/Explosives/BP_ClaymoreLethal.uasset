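; Claymore lethal equipment that places an explosive on the ground in front of its owner when released.
; A downward line trace ahead of the owner finds the spot and spawns ExplosiveToSpawn there, yawed from the controller's rotation.
; A valid spawn triggers a client event that reduces lethal ammo through the owner, while a missed trace shows a failure widget.
; The construction script sets the claymore UI icon on top of the parent's setup.
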(event `self.OnRelease`
  (`self.Spawn Claymore`))

(event `Spawn Claymore`
  (bind _returnvalue (`self.GetOwner`))
  (bind _returnvalue_2 (`self.GetOwner`))
  (bind (_returnvalue_roll _returnvalue_pitch _returnvalue_yaw) (`KismetMathLibrary.BreakRotator` (`Controller.GetControlRotation` (`self.GetInstigatorController` _returnvalue_2))))
  (bind _returnvalue_3 (+ (`self.K2_GetActorLocation` _returnvalue) (* (`self.GetActorForwardVector` _returnvalue) 100.0)))
  (bind _outhit (`KismetSystemLibrary.LineTraceSingle` _returnvalue_3 (+ _returnvalue_3 (* (`self.GetActorUpVector` _returnvalue) -200.0)) "TraceTypeQuery1" false (`|MakeArray` self :!type "Actor Object Reference")))
  (if (`GameplayStatics.BreakHitResult` _outhit)
    (bind _returnvalue_4 (`|SpawnActorFromClass` (`self.ExplosiveToSpawn`) (`KismetMathLibrary.MakeTransform` (`.Location` (`GameplayStatics.BreakHitResult` _outhit)) (`KismetMathLibrary.MakeRotator` 0.0 0.0 (- _returnvalue_yaw 90.0))) "Undefined" "OverrideRootScale" _returnvalue_2 (cast `Pawn` _returnvalue_2 :!pure true)))
    (`/Engine/EditorBlueprintResources/StandardMacros.IsValid` _returnvalue_4
      (:`Is Valid`
        (`self.Client_ReduceLethalAmmo`)))
    (else
      (`self.Client_ShowFailMessage`))))

(event `Client_ReduceLethalAmmo`
  (message `/Game/FPS/Blueprints/Interfaces/iPawnActions.ReduceLethalAmmo` (`self.GetOwner`)))

(event `Client_ShowFailMessage`
  (bind _returnvalue (`|CreateWidget` "/Game/FPS/UI/Gameplay/WB_ClaymoreFailmessage.WB_ClaymoreFailmessage_C" (`GameplayStatics.GetPlayerController` 0)))
  (`UserWidget.AddToViewport` _returnvalue 0))

(fn `UserConstructionScript`
  (`parent.UserConstructionScript`)
  (set `self.UI_Icon` "/Game/FPS/UI/Textures/T_Claymore.T_Claymore"))