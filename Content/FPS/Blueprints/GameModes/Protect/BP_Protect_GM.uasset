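; BP_Protect_GM is the game mode for the Protect mode, adding staged spawn points and a boss bot.
; ActivateNewSpawns enables only the Team A and B spawns whose State matches the given value.
; SpawnBossBot spawns one boss AI for team 1 at a random eligible Team B spawn, marks that spawn unusable and registers its controller.
; It then copies both teams' bot controller lists to BP_Base_GS.
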(event `self.ReceiveBeginPlay`
  (`parent.ReceiveBeginPlay`))

(event `ActivateNewSpawns`
  (params (NewParam :type Integer))
  ;[1 1 1] Activate New Spawns
  (for _array_element (`self.PlayerSpawnsA`)
    (set `/Game/FPS/Blueprints/PlayerSpawn/BP_PlayerSpawn.bActive` (== NewParam (`/Game/FPS/Blueprints/PlayerSpawn/BP_PlayerSpawn.State` _array_element)) _array_element))
  (for _array_element_2 (`self.PlayerSpawnsB`)
    (set `/Game/FPS/Blueprints/PlayerSpawn/BP_PlayerSpawn.bActive` (== NewParam (`/Game/FPS/Blueprints/PlayerSpawn/BP_PlayerSpawn.State` _array_element_2)) _array_element_2)))

(event `SpawnBossBot`
  (`|ExecutionSequence`
    (:`then_0`
      (if (> 1 0)
        (for _ (range 1 2)
          (bind _posiblespawn (`self.TeamPosibleSpawn` 1 (`self.PlayerSpawnsB`)))
          (bind _bestspawns (`self.ChooseSpawn` _posiblespawn 1))
          (if (`KismetArrayLibrary.Array_IsValidIndex` _bestspawns)
            (bind _output_get (set `self.SelectedSpawn` (`|GetArrayItem` _bestspawns (`KismetMathLibrary.RandomIntegerInRange` 0 (`KismetArrayLibrary.Array_LastIndex` _bestspawns)))))
            (set `/Game/FPS/Blueprints/PlayerSpawn/BP_PlayerSpawn.bCanBeUsed` false _output_get)
            (bind (_returnvalue_location _returnvalue_rotation) (`KismetMathLibrary.BreakTransform` (`SceneComponent.K2_GetComponentToWorld` (`Actor.RootComponent` _output_get))))
            (bind _returnvalue (`AIBlueprintHelperLibrary.SpawnAIFromClass` "/Game/FPS/Blueprints/AI_Characters/PlayerAI/BP_AI_Character_Boss.BP_AI_Character_Boss_C" (`self.AI_BehaviorTree`) _returnvalue_location _returnvalue_rotation true null))
            (`KismetArrayLibrary.Array_AddUnique` (`self.TeamBBotsControllers`) (`Pawn.GetController` _returnvalue))
            (message `/Game/FPS/Blueprints/Interfaces/iPlayerState.SetTeam` (`Pawn.PlayerState` _returnvalue) 1)))))
    (:`then_1`
      (bind _asbp_base_gs (cast `/Game/FPS/Blueprints/GameModes/BP_Base_GS` (`GameplayStatics.GetGameState`)))
      (set `/Game/FPS/Blueprints/GameModes/BP_Base_GS.BotsTeamAControllers` (`self.TeamABotsControllers`) _asbp_base_gs)
      (set `/Game/FPS/Blueprints/GameModes/BP_Base_GS.BotsTeamBControllers` (`self.TeamBBotsControllers`) _asbp_base_gs))))

(fn `UserConstructionScript`
  (`parent.UserConstructionScript`))