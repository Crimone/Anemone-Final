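; BP_Rush_GM is the game mode for Rush, managing which player spawns are active.
; ActivateNewSpawns takes a state value and loops through both spawn arrays, PlayerSpawnsA and PlayerSpawnsB.
; It enables spawns whose State matches that value and disables all others.
; BeginPlay and the construction script only call their parent implementations.
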(event `self.ReceiveBeginPlay`
  (`parent.ReceiveBeginPlay`))

(event `ActivateNewSpawns`
  (params (NewParam :type Integer))
  ;[1 1 1] Activate New Spawns
  (for _array_element (`self.PlayerSpawnsA`)
    (set `/Game/FPS/Blueprints/PlayerSpawn/BP_PlayerSpawn.bActive` (== NewParam (`/Game/FPS/Blueprints/PlayerSpawn/BP_PlayerSpawn.State` _array_element)) _array_element))
  (for _array_element_2 (`self.PlayerSpawnsB`)
    (set `/Game/FPS/Blueprints/PlayerSpawn/BP_PlayerSpawn.bActive` (== NewParam (`/Game/FPS/Blueprints/PlayerSpawn/BP_PlayerSpawn.State` _array_element_2)) _array_element_2)))

(fn `UserConstructionScript`
  (`parent.UserConstructionScript`))