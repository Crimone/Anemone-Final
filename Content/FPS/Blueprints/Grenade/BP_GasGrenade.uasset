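; Gas grenade actor that opens a timed damaging gas cloud as soon as it spawns on the authority.
; It enlarges an overlap sphere and shows a visual sphere, then a timer collapses both and destroys the actor.
; Overlap starts a looping damage timer only for player pawn 0 on team 0, crediting that pawn's own controller; leaving clears it.
; Projectile velocity, warning and multicast effect functions are empty stubs.
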(event `self.ReceiveBeginPlay`
  ;[1 1 1] Begin Play
  (`/Engine/EditorBlueprintResources/ActorMacros.Switch Has Authority`
    (:`Authority`
      (`self.ExplodeGrenade`))))

(event `ExplodeGrenade`
  ;[1 1 1] Explode
  (if (not (`self.bExploded`))
    (`self.Explode` (`self.GetInstigatorController` (`self.Instigator`)))))

(event `Explode`
  (params (Instigator :type "Controller Object Reference"))
  (bind _spheredamage (`self.SphereDamage`))
  ;[1 1 1] Explode
  (set `PrimitiveComponent.bGenerateOverlapEvents` true _spheredamage)
  (`SphereComponent.SetSphereRadius` _spheredamage (`self.Radius`) true)
  (`SceneComponent.SetVisibility` (`self.Sphere1`) true false)
  (`KismetSystemLibrary.K2_SetTimerDelegate` (delegate `DestroyGas`) (`self.TimeToExplode`)))

(event `DestroyGas`
  (bind _spheredamage (`self.SphereDamage`))
  (set `PrimitiveComponent.bGenerateOverlapEvents` false _spheredamage)
  (`SphereComponent.SetSphereRadius` _spheredamage 0.0 true)
  (`SceneComponent.SetVisibility` (`self.Sphere1`) false false)
  (set `self.bExploded` true)
  (`self.K2_DestroyActor`))

(event `OnExploded`
  ;[1 1 1] On Exploded
)

(event `self.SphereDamage.OnComponentBeginOverlap`
  (params (OverlappedComponent :type "PrimitiveComponent Object Reference") (OtherActor :type "Actor Object Reference") (OtherComp :type "PrimitiveComponent Object Reference") (OtherBodyIndex :type Integer) (bFromSweep :type Boolean) (SweepResult :type "HitResult Structure (by ref)"))
  (if (== OtherActor (`GameplayStatics.GetPlayerPawn` 0))
    (bind _asbp_player_state (cast `/Game/FPS/Blueprints/PlayerState/BP_PlayerState` (`Controller.PlayerState` (`self.GetInstigatorController` OtherActor))))
    (if (== (`/Game/FPS/Blueprints/PlayerState/BP_PlayerState.Team` _asbp_player_state) 0)
      (bind _returnvalue (`KismetSystemLibrary.K2_SetTimerDelegate` (delegate `DamagePlayer`) 1.0 true))
      (set `self.DamageHandle` _returnvalue)
      (set `self.DamageHandlePlayer` (`/Game/FPS/Blueprints/FunctionLibrary/BP_FunctionLibrary.GetPlayerNameFromPlayerState` _asbp_player_state)))))

(event `DamagePlayer`
  (`GameplayStatics.ApplyDamage` (stale `self.SphereDamage.OnComponentBeginOverlap` OtherActor) 10.0 (`self.GetInstigatorController` (stale `self.SphereDamage.OnComponentBeginOverlap` OtherActor)) self "/Game/FPS/Blueprints/Weapons/DamageTypes/DT_Grenade.DT_Grenade_C")
  (`self.ForceNetUpdate`))

(event `self.SphereDamage.OnComponentEndOverlap`
  (params (OverlappedComponent :type "PrimitiveComponent Object Reference") (OtherActor :type "Actor Object Reference") (OtherComp :type "PrimitiveComponent Object Reference") (OtherBodyIndex :type Integer))
  (if (== OtherActor (`GameplayStatics.GetPlayerPawn` 0))
    (bind _asbp_player_state (cast `/Game/FPS/Blueprints/PlayerState/BP_PlayerState` (`Controller.PlayerState` (`self.GetInstigatorController` OtherActor))))
    (if (== (`/Game/FPS/Blueprints/PlayerState/BP_PlayerState.Team` _asbp_player_state) 0)
      (if (`KismetTextLibrary.EqualEqual_TextText` (`self.DamageHandlePlayer`) (`/Game/FPS/Blueprints/FunctionLibrary/BP_FunctionLibrary.GetPlayerNameFromPlayerState` _asbp_player_state))
        (`KismetSystemLibrary.K2_ClearAndInvalidateTimerHandle` (`self.DamageHandle`))))))

(fn `Multicast_PlayEffects`)

(fn `OnRep_bExploded`
  (`self.OnExploded`))

(fn `SetProjectileVelocity`)

(fn `UserConstructionScript`
  (`self.SetProjectileVelocity`))

(fn `Warn`
  (params (bShowWarning :type Boolean)))