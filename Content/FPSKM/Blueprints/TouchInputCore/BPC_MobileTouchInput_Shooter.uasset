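; Actor component that bridges a mobile shooter's touch UI to gameplay through dispatcher-style calls.
; Raw touch press, move and release events are forwarded to MainWidget.
; Init binds the widget's joystick axis and action button events, which the component re-broadcasts, splitting Fire into shoot or melee.
; BeginPlay is empty and the local-player-checked widget creation is disconnected, so nothing here assigns MainWidget at runtime.
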(event `self.ReceiveBeginPlay`
  ;[1 1 1] Event - BeginPlay
)

(event `Event Init`
  ;[1 1 1] Event - BeginPlay
  (`|ExecutionSequence`
    (:`then_0`
      (add `/Game/FPSKM/Blueprints/TouchInputCore/Widgets/Widget_MobileShootingMain.InputTouch Axis MoveForward` (`self.MainWidget`) (delegate `Event Axis MoveForward`))
      (add `/Game/FPSKM/Blueprints/TouchInputCore/Widgets/Widget_MobileShootingMain.InputTouch Axis MoveRight` (`self.MainWidget`) (delegate `Event Axis MoveRight`))
      (add `/Game/FPSKM/Blueprints/TouchInputCore/Widgets/Widget_MobileShootingMain.InputTouch Axis LookUp` (`self.MainWidget`) (delegate `Event Axis LookUp`))
      (add `/Game/FPSKM/Blueprints/TouchInputCore/Widgets/Widget_MobileShootingMain.InputTouch Axis Turn` (`self.MainWidget`) (delegate `Event Axis Turn`))
      (add `/Game/FPSKM/Blueprints/TouchInputCore/Widgets/Widget_MobileShootingMain.InputTouch Axis Fire` (`self.MainWidget`) (delegate `Event Axis Fire`)))
    (:`then_1`
      (add `/Game/FPSKM/Blueprints/TouchInputCore/Widgets/Widget_MobileShootingMain.OnPressed_Button_Fire` (`self.MainWidget`) (delegate `Event OnPressed_Button_Fire`))
      (add `/Game/FPSKM/Blueprints/TouchInputCore/Widgets/Widget_MobileShootingMain.OnReleased_Button_Fire` (`self.MainWidget`) (delegate `Event OnReleased_Button_Fire`))
      (add `/Game/FPSKM/Blueprints/TouchInputCore/Widgets/Widget_MobileShootingMain.OnPressed_Button_Reload` (`self.MainWidget`) (delegate `Event OnPressed_Button_Reload`)))
    (:`then_2`
      (add `/Game/FPSKM/Blueprints/TouchInputCore/Widgets/Widget_MobileShootingMain.OnPressed_Button_Jump` (`self.MainWidget`) (delegate `Event OnPressed_Button_Jump`))
      (add `/Game/FPSKM/Blueprints/TouchInputCore/Widgets/Widget_MobileShootingMain.OnReleased_Button_Jump` (`self.MainWidget`) (delegate `Event OnReleased_Button_Jump`)))
    (:`then_3`
      (add `/Game/FPSKM/Blueprints/TouchInputCore/Widgets/Widget_MobileShootingMain.OnPressed_Button_Crouch` (`self.MainWidget`) (delegate `Event OnPressed_Button_Crouch`))
      (add `/Game/FPSKM/Blueprints/TouchInputCore/Widgets/Widget_MobileShootingMain.OnReleased_Button_Crouch` (`self.MainWidget`) (delegate `Event OnReleased_Button_Crouch`))
      (add `/Game/FPSKM/Blueprints/TouchInputCore/Widgets/Widget_MobileShootingMain.OnPressed_Button_Aim` (`self.MainWidget`) (delegate `Event OnPressed_Button_Aim`)))
    (:`then_4`
      (add `/Game/FPSKM/Blueprints/TouchInputCore/Widgets/Widget_MobileShootingMain.OnStart_SprintInput` (`self.MainWidget`) (delegate `Event OnStart_SprintInput`))
      (add `/Game/FPSKM/Blueprints/TouchInputCore/Widgets/Widget_MobileShootingMain.OnEnd_SprintInput` (`self.MainWidget`) (delegate `Event OnEnd_SprintInput`)))
    (:`then_5`
      (add `/Game/FPSKM/Blueprints/TouchInputCore/Widgets/Widget_MobileShootingMain.OnPressed_Button_WeaponSlot1` (`self.MainWidget`) (delegate `Event OnPressed_Button_WeaponSlot1`))
      (add `/Game/FPSKM/Blueprints/TouchInputCore/Widgets/Widget_MobileShootingMain.OnPressed_Button_WeaponSlot2` (`self.MainWidget`) (delegate `Event OnPressed_Button_WeaponSlot2`)))
    (:`then_6`
      (add `/Game/FPSKM/Blueprints/TouchInputCore/Widgets/Widget_MobileShootingMain.OnPressed_Button_GrenadeSlot` (`self.MainWidget`) (delegate `Event OnPressed_Button_GrenadeSlot`))
      (add `/Game/FPSKM/Blueprints/TouchInputCore/Widgets/Widget_MobileShootingMain.OnReleased_Button_GrenadeSlot` (`self.MainWidget`) (delegate `Event OnReleased_Button_GrenadeSlot`))
      (add `/Game/FPSKM/Blueprints/TouchInputCore/Widgets/Widget_MobileShootingMain.OnPressed_Button_Skill` (`self.MainWidget`) (delegate `Event OnPressed_Button_Skill`))
      (add `/Game/FPSKM/Blueprints/TouchInputCore/Widgets/Widget_MobileShootingMain.OnPressed_Button_Pause` (`self.MainWidget`) (delegate `Event OnPressed_Button_Pause`)))
    (:`then_7`
      (add `/Game/FPSKM/Blueprints/TouchInputCore/Widgets/Widget_MobileShootingMain.OnPressed_Button_TPP` (`self.MainWidget`) (delegate `Event OnPressed_Button_TPP`))
      (add `/Game/FPSKM/Blueprints/TouchInputCore/Widgets/Widget_MobileShootingMain.OnPressed_Button_LeanLeft` (`self.MainWidget`) (delegate `Event OnPressed_Button_LeanLeft`))
      (add `/Game/FPSKM/Blueprints/TouchInputCore/Widgets/Widget_MobileShootingMain.OnPressed_Button_LeanRight` (`self.MainWidget`) (delegate `Event OnPressed_Button_LeanRight`)))
    (:`then_8`
      (add `/Game/FPSKM/Blueprints/TouchInputCore/Widgets/Widget_MobileShootingMain.OnPressed_Button_Pick` (`self.MainWidget`) (delegate `Event OnPressed_Button_Pickup`))
      (add `/Game/FPSKM/Blueprints/TouchInputCore/Widgets/Widget_MobileShootingMain.OnReleased_Button_Pick` (`self.MainWidget`) (delegate `Event OnReleased_Button_Pickup`)))))

(event `Event Axis MoveForward`
  (params (AxisValue :type "Float (double-precision)") (JoystickAngle :type "Float (double-precision)") (JoystickMoveLength :type "Float (double-precision)"))
  ;[1 1 1] Event - BeginPlay
  (`self.InputTouch Axis MoveForward` AxisValue JoystickAngle JoystickMoveLength))

(event `Event Axis MoveRight`
  (params (AxisValue :type "Float (double-precision)"))
  ;[1 1 1] Event - BeginPlay
  (`self.InputTouch Axis MoveRight` AxisValue))

(event `Event Axis LookUp`
  (params (AxisValue :type "Float (double-precision)"))
  ;[1 1 1] Event - BeginPlay
  (`self.InputTouch Axis LookUp` AxisValue))

(event `Event Axis Turn`
  (params (AxisValue :type "Float (double-precision)"))
  ;[1 1 1] Event - BeginPlay
  (`self.InputTouch Axis Turn` AxisValue))

(event `Event Axis Fire`
  ;[1 1 1] Event - BeginPlay
  (`self.InputTouch Axis Fire`))

(event `Event OnPressed_Button_Fire`
  (params (Melee :type Boolean))
  ;[1 1 1] Event - BeginPlay
  (if Melee
    (`self.OnPressed Button Melee`)
    (else
      (`self.OnPressed Button Fire`))))

(event `Event OnReleased_Button_Fire`
  (params (Melee :type Boolean))
  ;[1 1 1] Event - BeginPlay
  (if Melee
    (`self.OnReleased Button Melee`)
    (else
      (`self.OnReleased Button Fire`))))

(event `Event OnPressed_Button_Reload`
  ;[1 1 1] Event - BeginPlay
  (`self.OnPressed Button Reload`))

(event `Event OnPressed_Button_Jump`
  ;[1 1 1] Event - BeginPlay
  (`self.OnPressed Button Jump`))

(event `Event OnPressed_Button_Crouch`
  ;[1 1 1] Event - BeginPlay
  (`self.OnPressed Button Crouch`))

(event `Event OnPressed_Button_Aim`
  ;[1 1 1] Event - BeginPlay
  (`self.OnPressed Button Aim`))

(event `Event OnReleased_Button_Jump`
  ;[1 1 1] Event - BeginPlay
  (`self.OnReleased Button Jump`))

(event `Event OnReleased_Button_Crouch`
  ;[1 1 1] Event - BeginPlay
  (`self.OnReleased Button Crouch`))

(event `Event OnStart_SprintInput`
  ;[1 1 1] Event - BeginPlay
  (`self.OnStart Sprint Input`))

(event `Event OnEnd_SprintInput`
  ;[1 1 1] Event - BeginPlay
  (`self.OnEnd Sprint Input`))

(event `Event OnPressed_Button_WeaponSlot1`
  ;[1 1 1] Event - BeginPlay
  (`self.OnPressed Button WeaponSlot1`))

(event `Event OnPressed_Button_WeaponSlot2`
  ;[1 1 1] Event - BeginPlay
  (`self.OnPressed Button WeaponSlot2`))

(event `Event OnPressed_Button_GrenadeSlot`
  ;[1 1 1] Event - BeginPlay
  (`self.OnPressed_Button_GrenadeSlot`))

(event `Event OnPressed_Button_TPP`
  ;[1 1 1] Event - BeginPlay
  (`self.OnPressed_Button_TPP`))

(event `Event OnPressed_Button_LeanLeft`
  ;[1 1 1] Event - BeginPlay
  (`self.OnPressed_Button_LeanLeft`))

(event `Event OnPressed_Button_LeanRight`
  ;[1 1 1] Event - BeginPlay
  (`self.OnPressed_Button_LeanRight`))

(event `Event OnPressed_Button_Pickup`
  ;[1 1 1] Event - BeginPlay
  (`self.OnPressed Button Pickup`))

(event `Event OnReleased_Button_Pickup`
  ;[1 1 1] Event - BeginPlay
  (`self.OnReleased Button Pickup`))

(event `Event OnReleased_Button_GrenadeSlot`
  ;[1 1 1] Event - BeginPlay
  (`self.OnReleased_Button_GrenadeSlot`))

(event `Event OnPressed_Button_Skill`
  ;[1 1 1] Event - BeginPlay
  (`self.OnPressed_Button_Skill`))

(event `Event OnPressed_Button_Pause`
  ;[1 1 1] Event - BeginPlay
  (`self.OnPressed_Button_Pause`))

(event `/Game/FPSKM/Blueprints/TouchInputCore/TouchInputInterface.OnPressed_InputTouch`
  (params (Location :type "Vector Structure") (FingerIndex :type Byte))
  ;[1 1 1] Input Touch Events
  (bind _mainwidget (`self.MainWidget`)
    (:`then`
      (`/Game/FPSKM/Blueprints/TouchInputCore/TouchInputInterface.OnPressed_InputTouch` _mainwidget Location FingerIndex))
    (:`else`)))

(event `/Game/FPSKM/Blueprints/TouchInputCore/TouchInputInterface.OnReleased_InputTouch`
  (params (Location :type "Vector Structure") (FingerIndex :type Byte))
  ;[1 1 1] Input Touch Events
  (bind _mainwidget (`self.MainWidget`)
    (:`then`
      (`/Game/FPSKM/Blueprints/TouchInputCore/TouchInputInterface.OnReleased_InputTouch` _mainwidget Location FingerIndex))
    (:`else`)))

(event `/Game/FPSKM/Blueprints/TouchInputCore/TouchInputInterface.OnMoved_InputTouch`
  (params (Location :type "Vector Structure") (FingerIndex :type Byte))
  ;[1 1 1] Input Touch Events
  (bind _mainwidget (`self.MainWidget`)
    (:`then`
      (`/Game/FPSKM/Blueprints/TouchInputCore/TouchInputInterface.OnMoved_InputTouch` _mainwidget Location FingerIndex))
    (:`else`)))